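; BP_Scientist is a controllable pawn that moves along fixed world axes from player input.
; The UPdown axis feeds movement input along world Y and LeftRight along world X.
; While either axis is non-zero, Tick turns the Cube component toward the input direction with a shortest-path rotator lerp scaled by delta time and RotationSpeed.
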(event `InputAxis|UPdown`
  (params (AxisValue :type "Float (single-precision)"))
  (`self.AddMovementInput` (0.0 1.0 0.0) AxisValue))

(event `InputAxis|LeftRight`
  (params (AxisValue :type "Float (single-precision)"))
  (`self.AddMovementInput` (1.0 0.0 0.0) AxisValue))

(event `self.ReceiveTick`
  (params (DeltaSeconds :type "Float (single-precision)"))
  (if (or (!= (`self.GetInputAxisValue`) 0.0) (!= (`self.GetInputAxisValue`) 0.0))
    (set `self.direction` (`KismetMathLibrary.MakeVector` (`self.GetInputAxisValue`) (`self.GetInputAxisValue`)))
    (`SceneComponent.K2_SetWorldRotation` (`self.Cube`) (`KismetMathLibrary.RLerp` (`SceneComponent.K2_GetComponentRotation` (`self.Cube`)) (`KismetMathLibrary.Conv_VectorToRotator` (`self.direction`)) (* DeltaSeconds (`self.rotationSpeed`)) true) false false)))

(fn `UserConstructionScript`)